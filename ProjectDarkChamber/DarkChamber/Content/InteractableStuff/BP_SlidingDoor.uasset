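; Interactable sliding door that moves its SlidingDoor component between positions A and B on a Timeline.
; Activate drives Interaction and Lever doors, while ChangeDoorState drives Statue doors, skipping the parent Activate call.
; Both paths call the parent Interact, then play or reverse the Timeline based on IsOpen.
; The Reverse flag starts the door at B and swaps the lerp endpoints.
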(event `self.Activate`
  (bind _dooropentype (`self.doorOpenType`))
  ;[1 0.6438 0.3368] Check if door is open/closed
  (if (or (`|EnumEquality` _dooropentype "Interaction") (`|EnumEquality` _dooropentype "Lever"))
    (`parent.Activate`)
    (`parent.Interact` null :!label _label)
    (if (`self.isOpen`)
      (bind (_direction _newtrack_0) (`Timeline|Timeline` :!label _label_2)
        (:`Update`
          (if (`self.reverse`)
            ;[0.8473 1 0.3385] Slide Door Reverse
            (`SceneComponent.K2_SetRelativeLocationAndRotation` :`self` (`self.SlidingDoor`) :`NewLocation` (`KismetMathLibrary.VLerp` (`self.B`) (`self.A`) _newtrack_0))
            (else
              ;[0.5927 1 0.4055] Slide Door Normaly
              (`SceneComponent.K2_SetRelativeLocationAndRotation` :`self` (`self.SlidingDoor`) :`NewLocation` (`KismetMathLibrary.VLerp` (`self.A`) (`self.B`) _newtrack_0))))))
      (else
        (goto _label_2 :!via `Reverse`)))))

(event `self.ChangeDoorState`
  ;[1 0.6438 0.3368] Check if door is open/closed
  (if (`|EnumEquality` (`self.doorOpenType`) "Statue")
    (goto _label)))

(event `self.ReceiveBeginPlay`
  ;[1 0 0 0.09] Begin Play
  (if (!= (`self.reverse`) false)
    (`SceneComponent.K2_SetRelativeLocationAndRotation` :`self` (`self.SlidingDoor`) :`NewLocation` (`self.B`))))

(fn `UserConstructionScript`)