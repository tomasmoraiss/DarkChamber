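; Interactable statue that turns a further 90 degrees each time an actor interacts with it.
; Interact calls its parent, then a timeline lerps the actor's rotation along the shortest path from the stored start rotation to that offset.
; CanInteract blocks re-triggering during the turn; on finish the new rotation is stored as the next start, as it is on BeginPlay.
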(event `self.Interact`
  (params (ActorInteracting :type "Actor Object Reference"))
  (bind _a (`self.A`))
  (`parent.Interact` ActorInteracting)
  (if (`self.canInteract`)
    (set `self.canInteract` false)
    (bind (_direction _newtrack_0) (`Timeline|Timeline` :!via `PlayFromStart`)
      (:`Update`
        ;[0.3325 1 0.2904] Change Door Rotation
        (`self.K2_SetActorRotation` (`KismetMathLibrary.RLerp` _a (`KismetMathLibrary.ComposeRotators` _a (struct :`Yaw` 90.0)) _newtrack_0 true)))
      (:`Finished`
        (set `self.A` (`self.K2_GetActorRotation`) :!label _label)
        (set `self.canInteract` true)))))

(event `self.ReceiveBeginPlay`
  (goto _label))

(fn `UserConstructionScript`)