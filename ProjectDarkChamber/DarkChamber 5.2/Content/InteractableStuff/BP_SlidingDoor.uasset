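; BP_SlidingDoor is an interactable door that slides vertically between a raised position and a lowered one.
; Its DoorOpenType decides the trigger: Activate drives it in Interaction mode, while ChangeDoorState drives it in Statue mode.
; Both paths call the parent's Interact, then play or reverse a timeline based on IsOpen, lerping the SlidingDoor's relative location.
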(event `self.Activate`
  ;[1 0.6438 0.3368] Check if door is open/closed
  (if (`|EnumEquality` (`self.doorOpenType`) "Interaction")
    (`parent.Activate`)
    (`parent.Interact` null :!label _label)
    (if (`self.isOpen`)
      (bind (_direction _newtrack_0) (`Timeline|Timeline` :!label _label_2)
        (:`Update`
          ;[0.5927 1 0.4055] Slide Door
          (`SceneComponent.K2_SetRelativeLocationAndRotation` :`self` (`self.SlidingDoor`) :`NewLocation` (`KismetMathLibrary.VLerp` (0.0 250.0 -5.0) (0.0 250.0 -700.0) _newtrack_0))))
      (else
        (goto _label_2 :!via `Reverse`)))))

(event `self.ChangeDoorState`
  ;[1 0.6438 0.3368] Check if door is open/closed
  (if (`|EnumEquality` (`self.doorOpenType`) "Statue")
    (goto _label)))

(fn `UserConstructionScript`)