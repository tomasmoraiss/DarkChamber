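; Interactable wooden door that swings between its starting rotation and an offset open rotation.
; BeginPlay caches the starting rotation and a combined offset rotation as the two endpoints.
; Interact calls the parent implementation, then plays or reverses a Timeline based on IsOpen, which this Blueprint only reads.
; The Timeline track drives a shortest-path rotator lerp that sets the actor's rotation.
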(event `self.Interact`
  (params (ActorInteracting :type "Actor Object Reference"))
  ;[1 0.6438 0.3368] Check if door is open/closed
  (`parent.Interact` null)
  (if (`self.isOpen`)
    (bind (_direction _newtrack_0) (`Timeline|Timeline` :!label _label)
      (:`Update`
        ;[0.3325 1 0.2904] Change Door Rotation
        (`self.K2_SetActorRotation` (`KismetMathLibrary.RLerp` (`self.A`) (`self.B`) _newtrack_0 true))))
    (else
      (goto _label :!via `Reverse`))))

(event `self.ReceiveBeginPlay`
  (bind _returnvalue (`self.K2_GetActorRotation`))
  (set `self.A` _returnvalue)
  (set `self.B` (`KismetMathLibrary.ComposeRotators` _returnvalue (struct :`Yaw` 75.0))))

(fn `UserConstructionScript`)